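; Game mode for a last-player-standing match with NPCs, spawned at random reachable points on BeginPlay.
; OnHumanDeath credits the attacker's kill count, marks player victims dead in their PlayerState, then checks for a sole survivor.
; A winner ends the game once, printing the highest kill count.
; Bomb triggers record the bomb on the PlayerState, check for a winner and damage the pawn; the light bar trigger is empty.
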(event `self.ReceiveBeginPlay`
  (`self.SpawnNPC` (`self.NPCSpawnCount`))
  (bind _outactors (`GameplayStatics.GetAllActorsOfClass` "/Game/BluePrints/InGame/ENV/BP_LightBar.BP_LightBar_C"))
  (set `self.LightBarCount` (`KismetArrayLibrary.Array_Length` _outactors)))

(fn `CheckWinner`
  (if (not (`self.bIsGameOver`))
    ; 승자 유무 판단
    (`/Engine/EditorBlueprintResources/StandardMacros.IsValid` (`self.GetWinner`)
      (:`Is Valid`
        (`|ExecutionSequence`
          (:`then_0`
            (set `self.bIsGameOver` true))
          (:`then_1`
            (`self.EndGame`)))))))

(fn `EndGame`
  (bind _player (`self.GetMostKillPlayer`))
  (`KismetSystemLibrary.PrintString` "GameOver")
  (`/Engine/EditorBlueprintResources/StandardMacros.IsValid` _player
    (:`Is Valid`
      (`KismetSystemLibrary.PrintText` (`|FormatText` "Max Kill Count {0}" (`/Game/BluePrints/InGame/Character/Player/BP_PlayerState.KillCount` _player))))
    (:`Is Not Valid`
      (`KismetSystemLibrary.PrintString` "Hello"))))

(fn `GetMostKillPlayer`
  (returns (Player :type "/Game/BluePrints/InGame/Character/Player/BP_PlayerState Object Reference"))
  (locals (BestKills :type Integer) (BestPlayer :type "/Game/BluePrints/InGame/Character/Player/BP_PlayerState Object Reference"))
  (`|ExecutionSequence`
    (:`then_0`
      ; 가장 많이 죽인 놈 찾기
      (for _array_element (`GameStateBase.PlayerArray` (`GameplayStatics.GetGameState`))
        (bind _asbp_player_state (cast `/Game/BluePrints/InGame/Character/Player/BP_PlayerState` _array_element))
        (bind _killcount (`/Game/BluePrints/InGame/Character/Player/BP_PlayerState.KillCount` _asbp_player_state))
        (if (> _killcount (`local.BestKills`))
          (set `local.BestKills` _killcount)
          (set `local.BestPlayer` _asbp_player_state))))
    (:`then_1`
      ; 가장 많이 죽인 놈 내보내기
      (return (`local.BestPlayer`)))))

(fn `GetWinner`
  (returns (Winner :type "/Game/BluePrints/InGame/Character/Player/BP_PlayerState Object Reference"))
  (locals (AliveCount :type Integer))
  (`|ExecutionSequence`
    (:`then_0`
      (for _array_element (`GameStateBase.PlayerArray` (`GameplayStatics.GetGameState`))
        (bind _asbp_player_state (cast `/Game/BluePrints/InGame/Character/Player/BP_PlayerState` _array_element))
        (if (not (`/Game/BluePrints/InGame/Character/Player/BP_PlayerState.bIsDead` _asbp_player_state))
          (`/Engine/EditorBlueprintResources/StandardMacros.IncrementInt` (`local.AliveCount`)))))
    (:`then_1`
      (if (== (`local.AliveCount`) 1)
        (for _array_element_2 (`GameStateBase.PlayerArray` (`GameplayStatics.GetGameState`))
          (bind _asbp_player_state_2 (cast `/Game/BluePrints/InGame/Character/Player/BP_PlayerState` _array_element_2))
          (if (not (`/Game/BluePrints/InGame/Character/Player/BP_PlayerState.bIsDead` _asbp_player_state_2))
            (return _asbp_player_state_2)))))
    (:`then_2`
      (if true
        _))))

(fn `OnHumanDeath`
  (params (Attacker :type "/Game/BluePrints/InGame/Character/Player/BP_Player Object Reference") (Victim :type "/Game/BluePrints/InGame/Character/BP_Human Object Reference"))
  (bind _playerstate (`/Game/BluePrints/InGame/Character/Player/BP_Player.GetBP_PlayerState` (`local.Attacker`)))
  (`/Engine/EditorBlueprintResources/StandardMacros.IsValid` Attacker
    (:`Is Valid`
      (`/Engine/EditorBlueprintResources/StandardMacros.IsValid` Victim
        (:`Is Valid`
          (`|ExecutionSequence`
            (:`then_0`
              ; 킬수 증가
              (`/Engine/EditorBlueprintResources/StandardMacros.IsValid` _playerstate
                (:`Is Valid`
                  (`/Engine/EditorBlueprintResources/StandardMacros.IncrementInt` (`/Game/BluePrints/InGame/Character/Player/BP_PlayerState.KillCount` _playerstate)))))
            (:`then_1`
              (bind _asbp_player (cast `/Game/BluePrints/InGame/Character/Player/BP_Player` (`local.Victim`)))
              (`self.OnPlayerDeath` (`/Game/BluePrints/InGame/Character/Player/BP_Player.GetBP_PlayerState` _asbp_player)))))))))

(fn `OnPlayerDeath`
  (params (PlayerState :type "/Game/BluePrints/InGame/Character/Player/BP_PlayerState Object Reference"))
  (set `/Game/BluePrints/InGame/Character/Player/BP_PlayerState.bIsDead` true PlayerState)
  (`self.CheckWinner`))

(fn `OnTriggerBomb`
  (params (PlayerState :type "/Game/BluePrints/InGame/Character/Player/BP_PlayerState Object Reference") (Bomb :type "/Game/BluePrints/InGame/ENV/BP_Bomb Object Reference"))
  (`/Engine/EditorBlueprintResources/StandardMacros.IsValid` PlayerState
    (:`Is Valid`
      (`/Engine/EditorBlueprintResources/StandardMacros.IsValid` Bomb
        (:`Is Valid`
          (`|ExecutionSequence`
            (:`then_0`
              (if (not (`BlueprintSetLibrary.Set_Contains` (`/Game/BluePrints/InGame/Character/Player/BP_PlayerState.Bombs` (`local.PlayerState`)) (`local.Bomb`)))
                (`BlueprintSetLibrary.Set_Add` (`/Game/BluePrints/InGame/Character/Player/BP_PlayerState.Bombs` (`local.PlayerState`)) (`local.Bomb`))))
            (:`then_1`
              (`self.CheckWinner`))
            (:`then_2`
              (bind _asbp_player (cast `/Game/BluePrints/InGame/Character/Player/BP_Player` (`PlayerState.GetPawn` (`local.PlayerState`))))
              (`GameplayStatics.ApplyDamage` _asbp_player 10.0 null (`local.Bomb`)))))))))

(fn `OnTriggerLightBar`)

(fn `SpawnNPC`
  (params (InNPCSpawnCount :type Integer))
  (for _ (range 1 (+ InNPCSpawnCount 1))
    (`|SpawnActorFromClass` "/Game/BluePrints/InGame/Character/NPC/BP_NPC.BP_NPC_C" (`KismetMathLibrary.MakeTransform` (`NavigationSystemV1.K2_GetRandomReachablePointInRadius` (0.0 0.0 300.0) 2000.0 null null)) "AdjustIfPossibleButAlwaysSpawn" "MultiplyWithRoot" null null)))

(fn `UserConstructionScript`)