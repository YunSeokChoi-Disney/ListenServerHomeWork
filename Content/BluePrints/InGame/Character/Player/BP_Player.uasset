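; BP_Player is the player character Blueprint, handling attack and sprint through client-to-server (C2S) and server-to-multicast (S2M) events.
; Attack input passes only from Idle, then the multicast sets the Attack state and plays a montage.
; Sprint input stores a flag, which a separate update event reads to multicast walk speed, passing zero when sprinting.
; GetSprintSpeed reduces sprint speed per player-state LightBar, floored at walk speed.
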(event `CallAttackInput`
  ; Attack
  (switch `/Game/BluePrints/InGame/Character/E_State` (`self.State`)
    (:`NewEnumerator0`
      (`self.C2S_Attack`))))

(event `CallSprintInput`
  (params (IsSprint :type Boolean))
  (`self.C2S_Sprint` IsSprint))

(event `C2S_Attack`
  ; Attack
  (switch `/Game/BluePrints/InGame/Character/E_State` (`self.State`)
    (:`NewEnumerator0`
      (`self.S2M_Attack`))))

(event `S2M_Sprint`
  (params (`New Walk Speed` :type "Float (double-precision)"))
  (set `CharacterMovementComponent.MaxWalkSpeed` `New Walk Speed` (`self.CharacterMovement`)))

(event `S2M_Attack`
  ; Attack
  (`|ExecutionSequence`
    (:`then_0`
      (set `self.State` "NewEnumerator1"))
    (:`then_1`
      (`|PlayMontage` (`self.Mesh`) "/Game/Assets/Animations/AM_Attack.AM_Attack"))))

(event `C2S_Sprint`
  (params (IsSprint :type Boolean))
  (set `self.Is Sprint` IsSprint))

(event `C2S_UpdateSpeed`
  (if (`self.Is Sprint`)
    (`self.S2M_Sprint` 0.0)
    (else
      (`self.S2M_Sprint` (`self.WalkSpeed`)))))

(fn `GetBP_PlayerState`
  (returns (PlayerState :type "/Game/BluePrints/InGame/Character/Player/BP_PlayerState Object Reference"))
  (bind _asbp_player_state (cast `/Game/BluePrints/InGame/Character/Player/BP_PlayerState` (`self.PlayerState`))
    (:`then`
      (return _asbp_player_state))
    (:`CastFailed`
      (return null))))

(fn `GetSprintSpeed`
  (returns (Speed :type "Float (double-precision)"))
  (locals (SprintSpeed :type "Float (double-precision)" :default 800.0))
  (bind _playerstate (`self.GetBP_PlayerState`))
  (`|ExecutionSequence`
    (:`then_0`
      (`/Engine/EditorBlueprintResources/StandardMacros.IsValid` _playerstate
        (:`Is Valid`
          (set `local.SprintSpeed` (- (`local.SprintSpeed`) (* (`BlueprintSetLibrary.Set_Length` (`/Game/BluePrints/InGame/Character/Player/BP_PlayerState.LightBars` _playerstate)) (`self.LightBarHandicap`)))))))
    (:`then_1`
      (return (`KismetMathLibrary.FMax` (`local.SprintSpeed`) (`self.WalkSpeed`))))))

(fn `UserConstructionScript`
  (`parent.UserConstructionScript`))